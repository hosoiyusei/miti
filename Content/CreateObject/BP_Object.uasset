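; BP_Object is an actor that can be destroyed while something overlaps its Box collision.
; BeginPlay enables query and physics collision on the Box, whose begin and end overlap events set and clear a Hit flag, with a "Hello" print on begin.
; A custom event named Event destroys the actor only while Hit is true; nothing in this Blueprint calls it.
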(event `self.ReceiveBeginPlay`
  (`PrimitiveComponent.SetCollisionEnabled` (`self.Box`) "QueryAndPhysics"))

(event `self.Box.OnComponentBeginOverlap`
  (params (OverlappedComponent :type "PrimitiveComponent Object Reference") (OtherActor :type "Actor Object Reference") (OtherComp :type "PrimitiveComponent Object Reference") (OtherBodyIndex :type Integer) (bFromSweep :type Boolean) (SweepResult :type "HitResult Structure (by ref)"))
  (set `self.bHit` true)
  (`KismetSystemLibrary.PrintString` "Hello"))

(event `self.Box.OnComponentEndOverlap`
  (params (OverlappedComponent :type "PrimitiveComponent Object Reference") (OtherActor :type "Actor Object Reference") (OtherComp :type "PrimitiveComponent Object Reference") (OtherBodyIndex :type Integer))
  (set `self.bHit` false))

(event `Event`
  (if (`self.bHit`)
    (`self.K2_DestroyActor`)))

(fn `UserConstructionScript`)