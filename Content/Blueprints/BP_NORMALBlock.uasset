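; BP_NORMALBlock is a colored block that changes material while the ThirdPersonCharacter overlaps its query-only Box trigger.
; SetColorEvent stores a Selection index and applies one of seven base color materials to the Cube.
; On begin overlap, SetColor swaps to that color's "_2" variant material; on end overlap, SetColorEvent restores the base material.
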(event `self.ReceiveBeginPlay`
  (`PrimitiveComponent.SetCollisionEnabled` (`self.Box`) "QueryOnly"))

(event `SetColorEvent`
  (params (Selection :type Integer))
  (bind _cube (`self.Cube`))
  (bind _output_get (set `self.Selection` Selection))
  (switch `int` _output_get
    (:`0`
      (`PrimitiveComponent.SetMaterial` _cube 0 "/Game/Material/MT_Red.MT_Red"))
    (:`1`
      (`PrimitiveComponent.SetMaterial` _cube 0 "/Game/Material/MT_Blue.MT_Blue"))
    (:`2`
      (`PrimitiveComponent.SetMaterial` _cube 0 "/Game/Material/MT_Green.MT_Green"))
    (:`3`
      (`PrimitiveComponent.SetMaterial` _cube 0 "/Game/Material/MT_Yellow.MT_Yellow"))
    (:`4`
      (`PrimitiveComponent.SetMaterial` _cube 0 "/Game/Material/MT_Orange.MT_Orange"))
    (:`5`
      (`PrimitiveComponent.SetMaterial` _cube 0 "/Game/Material/MT_rightBlue.MT_rightBlue"))
    (:`6`
      (`PrimitiveComponent.SetMaterial` _cube 0 "/Game/Material/MT_Purple.MT_Purple"))))

(event `self.Box.OnComponentBeginOverlap`
  (params (OverlappedComponent :type "PrimitiveComponent Object Reference") (OtherActor :type "Actor Object Reference") (OtherComp :type "PrimitiveComponent Object Reference") (OtherBodyIndex :type Integer) (bFromSweep :type Boolean) (SweepResult :type "HitResult Structure (by ref)"))
  (cast `/Game/ThirdPersonBP/Blueprints/ThirdPersonCharacter` OtherActor)
  (`self.SetColor`))

(event `self.Box.OnComponentEndOverlap`
  (params (OverlappedComponent :type "PrimitiveComponent Object Reference") (OtherActor :type "Actor Object Reference") (OtherComp :type "PrimitiveComponent Object Reference") (OtherBodyIndex :type Integer))
  (cast `/Game/ThirdPersonBP/Blueprints/ThirdPersonCharacter` OtherActor)
  (`self.SetColorEvent` (`self.Selection`)))

(event `SetColor`
  (bind _cube (`self.Cube`))
  (switch `int` (`self.Selection`)
    (:`0`
      (`PrimitiveComponent.SetMaterial` _cube 0 "/Game/Material/MT_Red_2.MT_Red_2"))
    (:`1`
      (`PrimitiveComponent.SetMaterial` _cube 0 "/Game/Material/MT_Blue_2.MT_Blue_2"))
    (:`2`
      (`PrimitiveComponent.SetMaterial` _cube 0 "/Game/Material/MT_Green_2.MT_Green_2"))
    (:`3`
      (`PrimitiveComponent.SetMaterial` _cube 0 "/Game/Material/MT_Yellow_2.MT_Yellow_2"))
    (:`4`
      (`PrimitiveComponent.SetMaterial` _cube 0 "/Game/Material/MT_Orange_2.MT_Orange_2"))
    (:`5`
      (`PrimitiveComponent.SetMaterial` _cube 0 "/Game/Material/MT_rightBlue_2.MT_rightBlue_2"))
    (:`6`
      (`PrimitiveComponent.SetMaterial` _cube 0 "/Game/Material/MT_Purple_2.MT_Purple_2"))))

(fn `UserConstructionScript`)