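; BP_Star is a collectible star wrapped in a film that the third-person character bursts on touch.
; Tick shrinks and destroys the hit film, then shrinks the star, dims its four point lights and makes it home in on the player via ProjectileMovement.
; When the homing star overlaps the player, it fills the first free of five StarPos slots on the character and destroys itself.
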(event `self.ReceiveTick`
  (params (DeltaSeconds :type "Float (single-precision)"))
  (if (`self.bPlayerStar`)
    (`self.YourStarEvent`)
    (else
      (`self.HitFilmEvent`)
      (`self.StarShrinkEvent`))))

(event `self.Film.OnComponentBeginOverlap`
  (params (OverlappedComponent :type "PrimitiveComponent Object Reference") (OtherActor :type "Actor Object Reference") (OtherComp :type "PrimitiveComponent Object Reference") (OtherBodyIndex :type Integer) (bFromSweep :type Boolean) (SweepResult :type "HitResult Structure (by ref)"))
  (cast `/Game/ThirdPersonBP/Blueprints/ThirdPersonCharacter` OtherActor)
  (`GameplayStatics.PlaySound2D` "/Game/wab/ぷにょん.ぷにょん" 1.0 1.0 0.0 null null)
  (set `self.bFilmHit` true)
  (set `RotatingMovementComponent.RotationRate` (struct :`Pitch` 100.0 :`Yaw` 100.0 :`Roll` 100.0) (`self.RotatingMovement`)))

(event `self.Star.OnComponentBeginOverlap`
  (params (OverlappedComponent :type "PrimitiveComponent Object Reference") (OtherActor :type "Actor Object Reference") (OtherComp :type "PrimitiveComponent Object Reference") (OtherBodyIndex :type Integer) (bFromSweep :type Boolean) (SweepResult :type "HitResult Structure (by ref)"))
  (bind _asthird_person_character (cast `/Game/ThirdPersonBP/Blueprints/ThirdPersonCharacter` OtherActor))
  (`GameplayStatics.PlaySound2D` "/Game/wab/システム決定音_11.システム決定音_11" 1.0 1.0 0.0 null null)
  (if (`self.bYourStar`)
    (if (not (`self.bPlayerStar`))
      (set `self.bPlayerStar` true))))

(fn `HitFilmEvent`
  (bind _filmsize (`self.FilmSize`))
  (`/Engine/EditorBlueprintResources/StandardMacros.IsValid` (`self.Film`)
    (:`Is Valid`
      (if (`self.bFilmHit`)
        (if (>= (`self.FilmSize`) 0.0)
          (set `self.FilmSize` (- (`self.FilmSize`) 0.1))
          (`SceneComponent.SetWorldScale3D` (`self.Film`) (`KismetMathLibrary.MakeVector` _filmsize _filmsize _filmsize))
          (else
            (`ActorComponent.K2_DestroyComponent` (`self.Film`))
            (set `self.bStarShrink` true)))))))

(fn `StarShrinkEvent`
  (bind _light_intensity (`self.Light intensity`))
  (bind _starsize (`self.StarSize`))
  (if (`self.bStarShrink`)
    (if (>= (`self.StarSize`) 2.0)
      (set `self.StarSize` (- (`self.StarSize`) 0.2))
      (`SceneComponent.SetWorldScale3D` (`self.Star`) (`KismetMathLibrary.MakeVector` _starsize _starsize _starsize))
      (`LightComponent.SetIntensity` (`self.PointLight`) _light_intensity)
      (`LightComponent.SetIntensity` (`self.PointLight1`) _light_intensity)
      (`LightComponent.SetIntensity` (`self.PointLight2`) _light_intensity)
      (`LightComponent.SetIntensity` (`self.PointLight3`) _light_intensity)
      (if (>= (`self.Light intensity`) 300.0)
        (set `self.Light intensity` (- (`self.Light intensity`) 300.0)))
      (else
        (`/Engine/EditorBlueprintResources/StandardMacros.DoOnce` false
          (:`Completed`
            (set `ProjectileMovementComponent.HomingTargetComponent` (`Character.CapsuleComponent` (cast `/Game/ThirdPersonBP/Blueprints/ThirdPersonCharacter` (`GameplayStatics.GetPlayerCharacter` 0) :!pure true)) (`self.ProjectileMovement`))
            (set `ProjectileMovementComponent.bIsHomingProjectile` true (`self.ProjectileMovement`))
            (set `ProjectileMovementComponent.HomingAccelerationMagnitude` 200.0 (`self.ProjectileMovement`))
            (set `ProjectileMovementComponent.bSimulationEnabled` true (`self.ProjectileMovement`))
            (set `RotatingMovementComponent.RotationRate` (struct :`Pitch` 300.0 :`Yaw` 300.0 :`Roll` 300.0) (`self.RotatingMovement`))
            (set `self.bYourStar` true)))))))

(fn `UserConstructionScript`)

(fn `YourStarEvent`
  (bind _starpos (`/Game/ThirdPersonBP/Blueprints/ThirdPersonCharacter.StarPos` (cast `/Game/ThirdPersonBP/Blueprints/ThirdPersonCharacter` (`GameplayStatics.GetPlayerCharacter` 0) :!pure true)))
  (if (`self.bPlayerStar`)
    (if (`self.bSetPos`)
      _
      (elif (`/Game/Blueprints/BP_StarSetPos.Pos1` _starpos)
        (if (`/Game/Blueprints/BP_StarSetPos.Pos2` _starpos)
          (if (`/Game/Blueprints/BP_StarSetPos.Pos3` _starpos)
            (if (`/Game/Blueprints/BP_StarSetPos.Pos4` _starpos)
              (if (not (`/Game/Blueprints/BP_StarSetPos.Pos5` _starpos))
                (`/Game/Blueprints/BP_StarSetPos.Star5` _starpos)
                (`self.K2_DestroyActor` :!label _label))
              (else
                (`/Game/Blueprints/BP_StarSetPos.Star4` _starpos)
                (goto _label)))
            (else
              (`/Game/Blueprints/BP_StarSetPos.Star3` _starpos)
              (goto _label)))
          (else
            (`/Game/Blueprints/BP_StarSetPos.Star2` _starpos)
            (goto _label)))
        (else
          (`/Game/Blueprints/BP_StarSetPos.Star1` _starpos)
          (goto _label))))))