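; BP_Goal is the level goal, which becomes active once the Pos5 flag on the player's StarPos reference is set.
; Tick caches StarPos from the ThirdPersonCharacter, then calls GoalEvent, which uses a DoOnce to start a delayed loop spawning light particles at the Sphere.
; When the character overlaps the Sphere with Pos5 set, it plays a clear sound once and calls Goal on ThirdPersonGameMode.
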(event `self.ReceiveTick`
  (params (DeltaSeconds :type "Float (single-precision)"))
  (bind _starpos (`/Game/ThirdPersonBP/Blueprints/ThirdPersonCharacter.StarPos` (cast `/Game/ThirdPersonBP/Blueprints/ThirdPersonCharacter` (`GameplayStatics.GetPlayerCharacter` 0) :!pure true)))
  (`/Engine/EditorBlueprintResources/StandardMacros.IsValid` (`self.NewVar_0`)
    (:`Is Valid`
      (`self.GoalEvent`))
    (:`Is Not Valid`
      (`/Engine/EditorBlueprintResources/StandardMacros.IsValid` _starpos
        (:`Is Valid`
          (set `self.NewVar_0` _starpos))))))

(event `GoalEvent`
  (if (`/Game/Blueprints/BP_StarSetPos.Pos5` (`self.NewVar_0`))
    (`/Engine/EditorBlueprintResources/StandardMacros.DoOnce` false
      (:`Completed`
        (`GameplayStatics.SpawnEmitterAtLocation` "/Game/Luos8Elements/Particles/Light/Par_4E_LightDef_01.Par_4E_LightDef_01" (`SceneComponent.K2_GetComponentLocation` (`self.Sphere`)) :!label _label)
        (`KismetSystemLibrary.Delay` 2.5)
        (if (not (`self.NewVar_1`))
          (goto _label))))))

(event `self.Sphere.OnComponentBeginOverlap`
  (params (OverlappedComponent :type "PrimitiveComponent Object Reference") (OtherActor :type "Actor Object Reference") (OtherComp :type "PrimitiveComponent Object Reference") (OtherBodyIndex :type Integer) (bFromSweep :type Boolean) (SweepResult :type "HitResult Structure (by ref)"))
  (if (`/Game/Blueprints/BP_StarSetPos.Pos5` (`self.NewVar_0`))
    (cast `/Game/ThirdPersonBP/Blueprints/ThirdPersonCharacter` OtherActor)
    (`/Engine/EditorBlueprintResources/StandardMacros.DoOnce` false
      (:`Completed`
        (`GameplayStatics.PlaySound2D` "/Game/wab/流れるようなゲームクリア音.流れるようなゲームクリア音" 1.0 1.0 0.0 null null)
        (`/Game/ThirdPersonBP/Blueprints/ThirdPersonGameMode.Goal` (cast `/Game/ThirdPersonBP/Blueprints/ThirdPersonGameMode` (`GameplayStatics.GetGameMode`) :!pure true))))))

(fn `UserConstructionScript`)