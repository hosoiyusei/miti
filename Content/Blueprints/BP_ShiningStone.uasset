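; BP_ShiningStone is a stone actor that stays in the level only if it lands on a BP_NORMALBlock shortly after spawning.
; When Sphere1 begins overlapping such a block, the Sphere component stops simulating physics, loses gravity and collision, and a Hit flag is set.
; A single delayed check from BeginPlay destroys the actor if Hit is still false.
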(event `self.ReceiveBeginPlay`
  (`KismetSystemLibrary.Delay` 2.0)
  (if (not (`self.bHit`))
    (`self.K2_DestroyActor`)))

(event `self.Sphere1.OnComponentBeginOverlap`
  (params (OverlappedComponent :type "PrimitiveComponent Object Reference") (OtherActor :type "Actor Object Reference") (OtherComp :type "PrimitiveComponent Object Reference") (OtherBodyIndex :type Integer) (bFromSweep :type Boolean) (SweepResult :type "HitResult Structure (by ref)"))
  (bind _sphere (`self.Sphere`))
  (cast `/Game/Blueprints/BP_NORMALBlock` OtherActor)
  (`PrimitiveComponent.SetSimulatePhysics` _sphere false)
  (`PrimitiveComponent.SetEnableGravity` _sphere false)
  (`PrimitiveComponent.SetCollisionEnabled` _sphere "NoCollision")
  (set `self.bHit` true))

(fn `UserConstructionScript`)