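; BP_StarSetPos is an actor that displays up to five collected stars at marker positions that follow the player.
; Tick moves its Sphere just above the player capsule and snaps each spawned star to its marker through a nested validity chain, so later stars depend on earlier ones.
; Star1–Star5 events each spawn a BP_NormalStar once and call StarPlus on the game mode's Play reference.
; Star5 also sets AllStarsAreComplete.
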(event `self.ReceiveTick`
  (params (DeltaSeconds :type "Float (single-precision)"))
  (bind _newvar_1 (`self.NewVar_1`))
  (bind _newvar_3 (`self.NewVar_3`))
  (bind _newvar_2 (`self.NewVar_2`))
  (bind _newvar_4 (`self.NewVar_4`))
  (bind _newvar_0 (`self.NewVar_0`))
  (bind (_returnvalue_x _returnvalue_y _returnvalue_z) (`KismetMathLibrary.BreakVector` (`SceneComponent.K2_GetComponentLocation` (`Character.CapsuleComponent` (cast `/Game/ThirdPersonBP/Blueprints/ThirdPersonCharacter` (`GameplayStatics.GetPlayerCharacter` 0) :!pure true)))))
  (`SceneComponent.K2_SetWorldLocation` (`self.Sphere`) (`KismetMathLibrary.MakeVector` _returnvalue_x _returnvalue_y (+ _returnvalue_z 20.0)) false false)
  (`/Engine/EditorBlueprintResources/StandardMacros.IsValid` _newvar_0
    (:`Is Valid`
      (`SceneComponent.K2_SetWorldLocation` (`/Game/Blueprints/BP_NormalStar.Star` _newvar_0) (`SceneComponent.K2_GetComponentLocation` (`self.Sphere1`)) false false)
      (`/Engine/EditorBlueprintResources/StandardMacros.IsValid` _newvar_1
        (:`Is Valid`
          (`SceneComponent.K2_SetWorldLocation` (`/Game/Blueprints/BP_NormalStar.Star` _newvar_1) (`SceneComponent.K2_GetComponentLocation` (`self.Sphere2`)) false false)
          (`/Engine/EditorBlueprintResources/StandardMacros.IsValid` _newvar_2
            (:`Is Valid`
              (`SceneComponent.K2_SetWorldLocation` (`/Game/Blueprints/BP_NormalStar.Star` _newvar_2) (`SceneComponent.K2_GetComponentLocation` (`self.Sphere3`)) false false)
              (`/Engine/EditorBlueprintResources/StandardMacros.IsValid` _newvar_3
                (:`Is Valid`
                  (`SceneComponent.K2_SetWorldLocation` (`/Game/Blueprints/BP_NormalStar.Star` _newvar_3) (`SceneComponent.K2_GetComponentLocation` (`self.Sphere4`)) false false)
                  (`/Engine/EditorBlueprintResources/StandardMacros.IsValid` _newvar_4
                    (:`Is Valid`
                      (`SceneComponent.K2_SetWorldLocation` (`/Game/Blueprints/BP_NormalStar.Star` _newvar_4) (`SceneComponent.K2_GetComponentLocation` (`self.Sphere5`)) false false))))))))))))

(event `Star1`
  (if (not (`self.Pos1`))
    (bind _returnvalue (`|SpawnActorFromClass` "/Game/Blueprints/BP_NormalStar.BP_NormalStar_C" (`SceneComponent.K2_GetComponentToWorld` (`self.Sphere1`)) "Undefined" "OverrideRootScale" null null))
    (set `self.NewVar_0` _returnvalue)
    (set `self.Pos1` true)
    (`/Game/Widget/WG_Play.StarPlus` (`/Game/ThirdPersonBP/Blueprints/ThirdPersonGameMode.Play` (cast `/Game/ThirdPersonBP/Blueprints/ThirdPersonGameMode` (`GameplayStatics.GetGameMode`) :!pure true)))))

(event `Star2`
  (if (not (`self.Pos2`))
    (bind _returnvalue (`|SpawnActorFromClass` "/Game/Blueprints/BP_NormalStar.BP_NormalStar_C" (`SceneComponent.K2_GetComponentToWorld` (`self.Sphere2`)) "Undefined" "OverrideRootScale" null null))
    (set `self.NewVar_1` _returnvalue)
    (set `self.Pos2` true)
    (`/Game/Widget/WG_Play.StarPlus` (`/Game/ThirdPersonBP/Blueprints/ThirdPersonGameMode.Play` (cast `/Game/ThirdPersonBP/Blueprints/ThirdPersonGameMode` (`GameplayStatics.GetGameMode`) :!pure true)))))

(event `Star3`
  (if (not (`self.Pos3`))
    (bind _returnvalue (`|SpawnActorFromClass` "/Game/Blueprints/BP_NormalStar.BP_NormalStar_C" (`SceneComponent.K2_GetComponentToWorld` (`self.Sphere3`)) "Undefined" "OverrideRootScale" null null))
    (set `self.NewVar_2` _returnvalue)
    (set `self.Pos3` true)
    (`/Game/Widget/WG_Play.StarPlus` (`/Game/ThirdPersonBP/Blueprints/ThirdPersonGameMode.Play` (cast `/Game/ThirdPersonBP/Blueprints/ThirdPersonGameMode` (`GameplayStatics.GetGameMode`) :!pure true)))))

(event `Star4`
  (if (not (`self.Pos4`))
    (bind _returnvalue (`|SpawnActorFromClass` "/Game/Blueprints/BP_NormalStar.BP_NormalStar_C" (`SceneComponent.K2_GetComponentToWorld` (`self.Sphere4`)) "Undefined" "OverrideRootScale" null null))
    (set `self.NewVar_3` _returnvalue)
    (set `self.Pos4` true)
    (`/Game/Widget/WG_Play.StarPlus` (`/Game/ThirdPersonBP/Blueprints/ThirdPersonGameMode.Play` (cast `/Game/ThirdPersonBP/Blueprints/ThirdPersonGameMode` (`GameplayStatics.GetGameMode`) :!pure true)))))

(event `Star5`
  (if (not (`self.Pos5`))
    (bind _returnvalue (`|SpawnActorFromClass` "/Game/Blueprints/BP_NormalStar.BP_NormalStar_C" (`SceneComponent.K2_GetComponentToWorld` (`self.Sphere5`)) "Undefined" "OverrideRootScale" null null))
    (set `self.NewVar_4` _returnvalue)
    (set `self.Pos5` true)
    (set `self.AllStarsAreComplete` true)
    (`/Game/Widget/WG_Play.StarPlus` (`/Game/ThirdPersonBP/Blueprints/ThirdPersonGameMode.Play` (cast `/Game/ThirdPersonBP/Blueprints/ThirdPersonGameMode` (`GameplayStatics.GetGameMode`) :!pure true)))))

(fn `UserConstructionScript`)