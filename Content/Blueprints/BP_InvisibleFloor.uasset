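; Invisible floor actor that makes a BP_HomingFloor appear while the player character is nearby and removes it when the player leaves.
; Each Tick measures the distance from the player's capsule to its root against a fixed radius.
; Within range, it spawns one floor at a random offset around itself, keeps the reference and passes its Sphere to HomingEvent.
; Out of range, it calls DestroyEvent on that floor and destroys it.
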(event `self.ReceiveTick`
  (params (DeltaSeconds :type "Float (single-precision)"))
  (bind _returnvalue (`KismetMathLibrary.RandomFloatInRange` -200.0 200.0))
  (bind _defaultsceneroot (`self.DefaultSceneRoot`))
  (bind _newvar_0 (`self.NewVar_0`))
  (bind (_returnvalue_location _returnvalue_rotation _returnvalue_scale) (`KismetMathLibrary.BreakTransform` (`SceneComponent.K2_GetComponentToWorld` _defaultsceneroot)))
  (bind (_returnvalue_x _returnvalue_y _returnvalue_z) (`KismetMathLibrary.BreakVector` (`SceneComponent.K2_GetComponentLocation` _defaultsceneroot)))
  (if (< (`KismetMathLibrary.Vector_Distance` (`SceneComponent.K2_GetComponentLocation` (`Character.CapsuleComponent` (cast `/Game/ThirdPersonBP/Blueprints/ThirdPersonCharacter` (`GameplayStatics.GetPlayerCharacter` 0) :!pure true))) (`SceneComponent.K2_GetComponentLocation` (`self.DefaultSceneRoot`))) 1000.0)
    (`/Engine/EditorBlueprintResources/StandardMacros.IsValid` (`self.NewVar_0`)
      (:`Is Not Valid`
        (bind _returnvalue_2 (`|SpawnActorFromClass` "/Game/Blueprints/BP_HomingFloor.BP_HomingFloor_C" (`KismetMathLibrary.MakeTransform` (`KismetMathLibrary.MakeVector` (+ _returnvalue_x _returnvalue) (+ _returnvalue_y _returnvalue) (+ _returnvalue_z _returnvalue)) _returnvalue_rotation _returnvalue_scale) "Undefined" "OverrideRootScale" null null))
        (bind _output_get (set `self.NewVar_0` _returnvalue_2))
        (`/Game/Blueprints/BP_HomingFloor.HomingEvent` _output_get (`self.Sphere`))))
    (else
      (`/Engine/EditorBlueprintResources/StandardMacros.IsValid` _newvar_0
        (:`Is Valid`
          (`/Game/Blueprints/BP_HomingFloor.DestroyEvent` _newvar_0)
          (`self.K2_DestroyActor` _newvar_0))))))

(fn `UserConstructionScript`)