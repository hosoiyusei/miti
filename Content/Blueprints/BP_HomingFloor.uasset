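; BP_HomingFloor is a randomly colored cube that homes toward a target and turns into a BP_NORMALBlock on arrival.
; BeginPlay picks one of seven materials, and HomingEvent passes a target component to the ProjectileMovement.
; Tick checks the distance to the target, then spawns the block at the cube's transform with the same color and destroys the cube component.
; DestroyEvent removes the spawned block.
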(event `self.ReceiveBeginPlay`
  (bind _cube (`self.Cube`))
  (bind _output_get (set `self.ColorNum` (`KismetMathLibrary.RandomIntegerInRange` 0 6)))
  (switch `int` _output_get
    (:`0`
      (`PrimitiveComponent.SetMaterial` _cube 0 "/Game/Material/MT_Red.MT_Red"))
    (:`1`
      (`PrimitiveComponent.SetMaterial` _cube 0 "/Game/Material/MT_Blue.MT_Blue"))
    (:`2`
      (`PrimitiveComponent.SetMaterial` _cube 0 "/Game/Material/MT_Green.MT_Green"))
    (:`3`
      (`PrimitiveComponent.SetMaterial` _cube 0 "/Game/Material/MT_Yellow.MT_Yellow"))
    (:`4`
      (`PrimitiveComponent.SetMaterial` _cube 0 "/Game/Material/MT_Orange.MT_Orange"))
    (:`5`
      (`PrimitiveComponent.SetMaterial` _cube 0 "/Game/Material/MT_rightBlue.MT_rightBlue"))
    (:`6`
      (`PrimitiveComponent.SetMaterial` _cube 0 "/Game/Material/MT_Purple.MT_Purple"))))

(event `DestroyEvent`
  (bind _newvar_0 (`self.NewVar_0`))
  (`/Engine/EditorBlueprintResources/StandardMacros.IsValid` _newvar_0
    (:`Is Valid`
      (`self.K2_DestroyActor` _newvar_0))))

(event `self.ReceiveTick`
  (params (DeltaSeconds :type "Float (single-precision)"))
  (`/Engine/EditorBlueprintResources/StandardMacros.IsValid` (`self.Homing Target Component`)
    (:`Is Valid`
      (if (< (`KismetMathLibrary.Vector_Distance` (`SceneComponent.K2_GetComponentLocation` (`self.DefaultSceneRoot`)) (`SceneComponent.K2_GetComponentLocation` (`self.Homing Target Component`))) 10.0)
        (`/Engine/EditorBlueprintResources/StandardMacros.IsValid` (`self.Cube`)
          (:`Is Valid`
            (bind _returnvalue (`|SpawnActorFromClass` "/Game/Blueprints/BP_NORMALBlock.BP_NORMALBlock_C" (`SceneComponent.K2_GetComponentToWorld` (`self.Cube`)) "Undefined" "OverrideRootScale" null null))
            (bind _output_get (set `self.NewVar_0` _returnvalue))
            (`/Game/Blueprints/BP_NORMALBlock.SetColorEvent` _output_get (`self.ColorNum`))
            (`ActorComponent.K2_DestroyComponent` (`self.Cube`))))))))

(event `HomingEvent`
  (params (`Homing Target Component` :type "SceneComponent Object Reference"))
  (bind _output_get (set `self.Homing Target Component` `Homing Target Component`))
  (set `ProjectileMovementComponent.HomingTargetComponent` _output_get (`self.ProjectileMovement`)))

(fn `UserConstructionScript`)